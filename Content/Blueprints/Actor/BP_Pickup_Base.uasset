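; Base pickup actor that animates its spawn and plays spawn, ground-impact and destruction (consume) sounds.
; A timeline drives uniform scale and a height offset from the initial location, firing the impact sound once when elevation dips below the start.
; When the timeline finishes, it starts sinusoidal movement and rotation through functions defined outside these graphs.
; Tick applies the calculated location and rotation to the actor every frame.
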(event EventBeginPlay
  (Audio|PlaySoundatLocation (Variables|Default|GetSpawnSound) (Transformation|GetActorLocation) "0, 0, 0" 1.0 1.0 0.0 0 0 0 0)
  (bind (_direction _elevation _scale) (Timeline|PickupElevationTimeline Play)
    (:Update
      (bind _output_get (Variables|Default|SetElevation _elevation))
      (Variables|Default|SetScale _scale)
      (Variables|Default|SetCalculatedLocation (CallFunction|CalculateElevation _output_get))
      (Transformation|SetActorScale3D (Math|Vector|MakeVector (Variables|Default|GetScale) (Variables|Default|GetScale) (Variables|Default|GetScale)))
      (if (< (Variables|Default|GetElevation) -0.1)
        (Utilities|FlowControl|DoOnce false
          (:Completed
            (Audio|PlaySoundatLocation (Variables|Default|GetGroundImpackSound) (Transformation|GetActorLocation) "0, 0, 0" 1.0 1.0 0.0 0 0 0 0)))))
    (:Finished
      (Class|EffectActor|StartSinusoidalMovement)
      (Class|EffectActor|StartRotation))))

(event EventTick
  (params (DeltaSeconds :type Float%20%28single-precision%29))
  (Transformation|SetActorLocationAndRotation (Variables|Default|GetCalculatedLocation) (Variables|Default|GetCalculatedRotation)))

(event EventDestroyed
  (Audio|PlaySoundatLocation (Variables|Default|GetConsumeSound) (Transformation|GetActorLocation) "0, 0, 0" 1.0 1.0 0.0 0 0 0 0))

(fn ConstructionScript)

(fn CalculateElevation
  (params (A :type Float%20%28double-precision%29))
  (bind _initiallocation (Variables|Default|GetInitialLocation))
  (return (Math|Vector|MakeVector (.x _initiallocation) (.y _initiallocation) (+ (.z _initiallocation) (* A (Variables|Default|GetSpawnApex))))))